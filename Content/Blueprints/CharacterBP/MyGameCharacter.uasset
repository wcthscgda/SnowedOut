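; First-person player character for a survival game, handling movement, item pickup, sleep, and inventory and crafting menus.
; A camera line trace copies item data into the Game Instance inventory and destroys the actor; menus freeze the player.
; Tick uses Delays to update hunger and temperature, which drain health when low, while campfires warm and time-dilated sleep heals.
; BeginPlay spawns recipe actors to build the crafting struct array.
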(event `InputAction|Interact`
  (params (Key :type "Key Structure"))
  ;[1 1 1] When E is pressed, it traces to where we are looking and stores the hit actor in our inventory.
  (:`Pressed`
    (`self.TraceItem`)
    (`self.AddToInv`)))

(event `ToggleCraft`
  (bind _returnvalue (`GameplayStatics.GetPlayerController` 0))
  ;[1 1 1] Opens and closes crafting
  (if (`self.IsPlayerFrozen`) :!label _label
    (`self.UnfreezePlayer`)
    (`Widget.RemoveFromParent` (stale _returnvalue_2))
    (`WidgetBlueprintLibrary.SetInputMode_GameOnly` _returnvalue)
    (else
      (`self.FreezePlayer`)
      (bind _returnvalue_2 (`|CreateWidget` "/Game/Blueprints/UI/Crafting/Wgt_CraftMain.Wgt_CraftMain_C" _returnvalue))
      (`UserWidget.AddToViewport` _returnvalue_2 0)
      (set `/Game/Blueprints/Controller_BP.invButtonClicked_C` -1 (`self.ControllerBPData`))
      (`WidgetBlueprintLibrary.SetInputMode_GameAndUIEx` _returnvalue _returnvalue_2))))

(event `Toggle Inventory`
  (bind _returnvalue (`GameplayStatics.GetPlayerController` 0))
  ;[1 1 1] Open/Close Inventory
  (if (`self.IsPlayerFrozen`) :!label _label_2
    (`self.UnfreezePlayer`)
    (`Widget.RemoveFromParent` (stale _returnvalue_2))
    (`WidgetBlueprintLibrary.SetInputMode_GameOnly` _returnvalue)
    (else
      (`self.FreezePlayer`)
      (bind _returnvalue_2 (`|CreateWidget` "/Game/Blueprints/UI/Inventory/Wgt_InventoryMain.Wgt_InventoryMain_C" _returnvalue))
      (`UserWidget.AddToViewport` _returnvalue_2 0)
      (set `/Game/Blueprints/Controller_BP.invButtonClicked_C` -1 (`self.ControllerBPData`))
      (`WidgetBlueprintLibrary.SetInputMode_GameAndUIEx` _returnvalue _returnvalue_2))))

(event `InputAction|OpenInventory`
  (params (Key :type "Key Structure"))
  (:`Pressed`
    (goto _label_2)))

(event `InputAction|OpenCrafting`
  (params (Key :type "Key Structure"))
  (:`Pressed`
    (goto _label)))

(event `FreezePlayer`
  (bind _returnvalue (`GameplayStatics.GetPlayerController` 0))
  ;[1 1 1] Freeze/Unfreeze charecter move and look, enables mouse movement
  (`/Engine/EditorBlueprintResources/StandardMacros.DoOnce` false :!label _label_3
    (:`Completed`
      (set `PlayerController.bEnableMouseOverEvents` true _returnvalue)
      (set `PlayerController.bEnableClickEvents` true _returnvalue)
      (set `PlayerController.bShowMouseCursor` true _returnvalue)
      (set `self.IsPlayerFrozen` true)
      (`Controller.SetIgnoreLookInput` _returnvalue true)
      (`Controller.SetIgnoreMoveInput` _returnvalue true)
      (goto _label_4 :!via `Reset`))))

(event `UnfreezePlayer`
  (bind _returnvalue (`GameplayStatics.GetPlayerController` 0))
  ;[1 1 1] Freeze/Unfreeze charecter move and look, enables mouse movement
  (`/Engine/EditorBlueprintResources/StandardMacros.DoOnce` false :!label _label_4
    (:`Completed`
      (set `PlayerController.bEnableMouseOverEvents` false _returnvalue)
      (set `PlayerController.bEnableClickEvents` false _returnvalue)
      (set `PlayerController.bShowMouseCursor` false _returnvalue)
      (set `self.IsPlayerFrozen` false)
      (`Controller.SetIgnoreLookInput` _returnvalue false)
      (`Controller.SetIgnoreMoveInput` _returnvalue false)
      (goto _label_3 :!via `Reset`))))

(event `InputAxis|Forward_Backward`
  (params (AxisValue :type "Float (single-precision)"))
  ;[1 1 1] Basic Movement Inputs
  (if (`self.CanMove`)
    (`self.AddMovementInput` (`self.GetActorForwardVector`) AxisValue)))

(event `InputAxis|Rotate`
  (params (AxisValue :type "Float (single-precision)"))
  ;[1 1 1] Basic Movement Inputs
  (if (`self.CanMove`)
    (`self.AddControllerYawInput` AxisValue)))

(event `InputAction|Crouch`
  (params (Key :type "Key Structure"))
  ;[1 1 1] Basic Movement Inputs
  (:`Pressed`
    (if (`self.CanMove`)
      (`self.Crouch`)))
  (:`Released`
    (`self.UnCrouch`)))

(event `InputAxis|LookUpDown`
  (params (AxisValue :type "Float (single-precision)"))
  ;[1 1 1] Basic Movement Inputs
  (if (`self.CanMove`)
    (`self.AddControllerPitchInput` AxisValue)))

(event `InputAxis|Strafe`
  (params (AxisValue :type "Float (single-precision)"))
  ;[1 1 1] Basic Movement Inputs
  (if (`self.CanMove`)
    (`self.AddMovementInput` (`self.GetActorRightVector`) AxisValue)))

(event `InputAction|Run`
  (params (Key :type "Key Structure"))
  (bind _charactermovement (`self.CharacterMovement`))
  ;[1 1 1] Basic Movement Inputs
  (:`Pressed`
    (set `CharacterMovementComponent.MaxWalkSpeed` (`self.RunSpeed`) _charactermovement))
  (:`Released`
    (set `CharacterMovementComponent.MaxWalkSpeed` 400.0 _charactermovement)))

(event `InputAction|Jump`
  (params (Key :type "Key Structure"))
  ;[1 1 1] Basic Movement Inputs
  (:`Pressed`
    (if (`self.CanMove`)
      (`self.Jump`))))

(event `self.ReceiveBeginPlay`
  (`|ExecutionSequence`
    (:`then_0`
      (`|ExecutionSequence`
        (:`then_0`
          (set `self.InCamp` false))
        (:`then_1`
          (bind _ascontroller_bp (cast `/Game/Blueprints/Controller_BP` (`GameplayStatics.GetGameInstance`)))
          (set `self.ControllerBPData` _ascontroller_bp))
        (:`then_2`
          (set `self.CanMove` true))
        (:`then_3`
          (set `self.PlayerTemp` 100.0))))
    (:`then_1`
      (`self.SetupRecipeArray`))))

(event `InputAction|Sleep`
  (params (Key :type "Key Structure"))
  (:`Pressed`
    (`KismetSystemLibrary.Delay` 0.0001)
    (if (`self.InSleepBox`)
      (`/Engine/EditorBlueprintResources/StandardMacros.FlipFlop`
        (:`A`
          (set `self.CanMove` false)
          (`GameplayStatics.SetGlobalTimeDilation` 4.0))
        (:`B`
          (set `self.CanMove` true :!label _label_5)
          (`GameplayStatics.SetGlobalTimeDilation` 1.0)))
      (else
        (goto _label_5)))))

(event `InputAction|Sleep`
  (params (Key :type "Key Structure"))
  (:`Pressed`
    (`/Engine/EditorBlueprintResources/StandardMacros.Gate` true :!label _label_6
      (:`Exit`
        (set `self.InSleepBox` true)))))

(event `self.ReceiveActorBeginOverlap`
  (params (OtherActor :type "Actor Object Reference"))
  (`|ExecutionSequence`
    (:`then_0`
      (cast `/Game/TriggerBox_Blueprint` OtherActor)
      (goto _label_6 :!via `Open`))
    (:`then_1`
      (cast `/Game/Blueprints/CampFireTrigger_BP` OtherActor)
      (goto _label_7 :!via `Open`))
    (:`then_2`
      (`KismetSystemLibrary.Delay` 0.0001)
      (`/Engine/EditorBlueprintResources/StandardMacros.Gate` true :!label _label_7
        (:`Exit`
          (set `self.InCamp` true))))))

(event `self.ReceiveActorEndOverlap`
  (params (OtherActor :type "Actor Object Reference"))
  (`|ExecutionSequence`
    (:`then_0`
      (cast `/Game/TriggerBox_Blueprint` OtherActor)
      (`|ExecutionSequence`
        (:`then_0`
          (goto _label_6 :!via `Close`))
        (:`then_1`
          (set `self.InSleepBox` false))))
    (:`then_1`
      (cast `/Game/Blueprints/CampFireTrigger_BP` OtherActor)
      (`|ExecutionSequence`
        (:`then_0`
          (goto _label_7 :!via `Close`))
        (:`then_1`
          (set `self.InCamp` false))))))

(event `self.ReceiveTick`
  (params (DeltaSeconds :type "Float (single-precision)"))
  (bind _playertemp (`self.PlayerTemp`))
  (bind _currenthunger (`self.CurrentHunger`))
  (`|ExecutionSequence`
    (:`then_0`
      ;[1 1 1] Increases Current Health when sleeping
      (if (not (`self.CanMove`))
        (set `self.CurrentHealth` (+ (`self.CurrentHealth`) 0.1))))
    (:`then_1`
      ;[1 1 1] Slowly brings down the "PlayerTemp" when "CurrentTemp" is lower.
      (`KismetSystemLibrary.Delay` 5.0)
      (`|ExecutionSequence`
        (:`then_0`
          (`/Engine/EditorBlueprintResources/StandardMacros.CompareInt` (`KismetMathLibrary.FTrunc` (`self.PlayerTemp`)) (`KismetMathLibrary.FTrunc` (`/Game/Blueprints/Controller_BP.CurrentTemp` (`self.ControllerBPData`)))
            (:`>`
              (set `self.+?` false))
            (:`<`
              (set `self.+?` true)))
          (bind _output_get (set `self.PlayerTemp` (`KismetMathLibrary.FClamp` (`KismetMathLibrary.SelectFloat` (- _playertemp 2.0) (+ _playertemp 2.0) (not (`self.+?`))) 0.0 100.0))))
        (:`then_2`
          _))
      (`KismetSystemLibrary.PrintString` (`KismetStringLibrary.Conv_DoubleToString` _output_get))
      (`/Engine/EditorBlueprintResources/StandardMacros.CompareInt` 30 (`KismetMathLibrary.FTrunc` _output_get)
        (:`>`
          (set `self.TempBelowHealthy` true))
        (:`<`
          (set `self.TempBelowHealthy` false))))
    (:`then_2`
      ;[1 1 1] Increases player temperature if they are in the campfire area
      (`KismetSystemLibrary.Delay` 2.0)
      (if (`self.InCamp`)
        (set `self.PlayerTemp` (`KismetMathLibrary.FClamp` (+ (`self.PlayerTemp`) 2.0) 0.0 (`self.MaxTemp`)))))
    (:`then_4`
      ;[1 1 1] When Player Temp is to low player starts taking damage
      (if (`self.TempBelowHealthy`)
        (set `self.CurrentHealth` (- (`self.CurrentHealth`) 0.05))))
    (:`then_5`
      ;[1 1 1] Males Hunger go down
      (`KismetSystemLibrary.Delay` 1.0)
      (set `self.CurrentHunger` (- _currenthunger 1.0))
      ;[1 1 1] Lowers player health if hunger is 0
      (`/Engine/EditorBlueprintResources/StandardMacros.CompareFloat` _currenthunger
        (:`==`
          _)
        (:`<`
          _))
      (set `self.HungerBelowHealthy` true))
    (:`then_6`
      (if (`self.HungerBelowHealthy`)
        (set `self.CurrentHealth` (- (`self.CurrentHealth`) 0.05))))))

(fn `AddToInv`
  ;[1 1 1] Take the actor hit stored in the ActorTraced var and cast it into Bp_MasterItem
  (bind _asbp_master_item (cast `/Game/Blueprints/Actor/Items/Bp_MasterItem` (`self.ActorTraced`)))
  (bind (_itemname _weight _itemdetails _thumbnail _isstackable _itemclass _isedible _issnare _iscampfire) (break `/Game/Blueprints/Actor/Items/Str_ItemData` (`/Game/Blueprints/Actor/Items/Bp_MasterItem.S_ItemData` _asbp_master_item)))
  ;[1 1 1] Adds newly mad S item Data struct to our inventory which is an array of S Item Data
  (`KismetArrayLibrary.Array_Add` (`/Game/Blueprints/Controller_BP.Inventory_C` (`self.ControllerBPData`)) (make `/Game/Blueprints/Actor/Items/Str_ItemData` _itemname _weight _itemdetails _thumbnail _isstackable _itemclass _isedible _issnare _iscampfire))
  (`self.K2_DestroyActor` (`self.ActorTraced`)))

(fn `SetupRecipeArray`
  ;[1 1 1] spawning a bp_masterCraft so new recipes can be added dynamically
  (`|SpawnActorFromClass` "/Game/Blueprints/Actor/Crafting_logic/BP_masterCrafting.BP_masterCrafting_C" (`KismetMathLibrary.MakeTransform` (0.0 0.0 0.0)) "AlwaysSpawn" "OverrideRootScale" null null)
  ;[1 1 1] Set to -1 so the Ui is empty Null selected recipe
  (set `self.RecipeSelected1p` -1)
  ;[1 1 1] Getting bp_mastercrafting (should only be 1, master) then we get all children classes which is class array car below
  (bind _outactors (`GameplayStatics.GetAllActorsOfClass` "/Game/Blueprints/Actor/Crafting_logic/BP_masterCrafting.BP_masterCrafting_C"))
  ;[1 1 1] Spawning each recipe to a physical actor
  (for _array_element (`/Game/Blueprints/Actor/Crafting_logic/BP_masterCrafting.CraftingRecipeClasses` (`|GetArrayItem` _outactors))
    (bind _returnvalue (`|SpawnActorFromClass` _array_element (`KismetMathLibrary.MakeTransform` (0.0 0.0 0.0)) "AlwaysSpawn" "OverrideRootScale" null null))
    ;[1 1 1] Add each recipie into an array of BP_master crafting actors
    (`KismetArrayLibrary.Array_Add` (`self.RecipeActorsInLevel1p`) _returnvalue))
  ;[1 1 1] For each recipe that is now data accessable
  (for _array_element_2 (`self.RecipeActorsInLevel1p`)
    ;[1 1 1] Comment
    ;;[1 1 1] Making an array of Str_craftingMain structures so their data can be accesssed on a per class index basis
    ;;;[1 1 1] creating Id for it as a safety measure
    (bind _output_get (set `self.RecipeID` (+ (`self.RecipeID`) 0.01)))
    (bind (_recipename _details _itemthumbnail _isunlocked _itemclass _itemid _metal _wood _rope _plant _rawmeat _cloth _coals _itemsrequired _metalclass _woodclass _ropeclass _plantclass _rawmeatclass _clothclass _coalsclass _rawmeat2 _rawmeat2class _coals2 _coals2class) (break `/Game/Blueprints/Actor/Crafting_logic/Str_craftingMain` (`/Game/Blueprints/Actor/Crafting_logic/BP_masterCrafting.Str_CraftingRecipe` _array_element_2)))
    (`KismetArrayLibrary.Array_Add` (`self.CraftingRecipes1p`) (make `/Game/Blueprints/Actor/Crafting_logic/Str_craftingMain` _recipename _details _itemthumbnail _isunlocked _itemclass _output_get _metal _wood _rope _plant _rawmeat _cloth _coals _itemsrequired _metalclass _woodclass _ropeclass _plantclass _rawmeatclass _clothclass _coalsclass _rawmeat2 _rawmeat2class _coals2 _coals2class))))

(fn `TraceItem`
  (bind _first_person_camera (`self.First Person Camera`))
  (bind _returnvalue (`SceneComponent.K2_GetComponentLocation` _first_person_camera))
  ;[1 1 1] Trace from our view a length of max use
  (bind (_outhit _returnvalue_2) (`KismetSystemLibrary.LineTraceSingle` :`Start` _returnvalue :`End` (+ _returnvalue (* (`SceneComponent.GetForwardVector` _first_person_camera) (`self.MaxUseDistance`))) :`TraceChannel` "TraceTypeQuery1" :`DrawDebugType` "ForDuration"))
  ;[1 1 1] Store the hit actor in actor traced
  (if _returnvalue_2
    (set `self.ActorTraced` (`.HitActor` (`GameplayStatics.BreakHitResult` _outhit)))
    (else
      (set `self.ActorTraced` null))))

(fn `UserConstructionScript`)