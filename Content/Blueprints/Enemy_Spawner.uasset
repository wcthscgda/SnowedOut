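; Enemy spawner actor that spawns AI at night while the Enemy count is below a maximum.
; BeginPlay caches the first SimpleSky actor found in the level.
; The Spawn_Enemy event checks that sky's NightTime flag and counts all Enemy actors against MaxEnemies.
; When both checks pass, it spawns one AI at a random point inside the SpawnVolume bounds; nothing in this graph triggers the event.
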(event `Spawn_Enemy`
  (bind _spawn_volume (`self.Spawn Volume`))
  (bind _assimple_sky (cast `/Game/Blueprints/SimpleSky` (`self.SimpleSky`)))
  (if (`/Game/Blueprints/SimpleSky.NightTime` _assimple_sky)
    (bind _outactors (`GameplayStatics.GetAllActorsOfClass` "/Game/Blueprints/enemy.enemy_C"))
    (if (< (`KismetArrayLibrary.Array_Length` _outactors) (`self.Max_Enemies`))
      (`AIBlueprintHelperLibrary.SpawnAIFromClass` null null (`KismetMathLibrary.RandomPointInBoundingBox` (`SceneComponent.K2_GetComponentLocation` _spawn_volume) (`BoxComponent.GetScaledBoxExtent` _spawn_volume))))))

(event `self.ReceiveBeginPlay`
  (bind _outactors (`GameplayStatics.GetAllActorsOfClass` "/Game/Blueprints/SimpleSky.SimpleSky_C"))
  (set `self.SimpleSky` (`|GetArrayItem` _outactors)))

(fn `UserConstructionScript`)