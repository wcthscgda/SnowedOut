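; Enemy Blueprint that wanders the navmesh until PawnSensing spots a pawn, then moves toward it.
; Seeing a pawn sets Inrange, which is never cleared, and issues AI MoveTo on the target if its cast succeeds.
; Tick starts a move to a random nearby navigable point when neither Inrange nor Moving is set.
; Every wander outcome sets Moving true and nothing resets it, so wandering does not repeat once set.
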(event `self.PawnSensing.OnSeePawn`
  (params (Pawn :type "Pawn Object Reference"))
  (set `self.inrange` true)
  (bind _asthird_person_character (cast `` Pawn))
  (`|AIMoveTo` self (0.0 0.0 0.0) _asthird_person_character))

(event `self.ReceiveTick`
  (params (DeltaSeconds :type "Float (single-precision)"))
  (if (`self.inrange`)
    _
    (elif (not (`self.moving`))
      (`|AIMoveTo` self (`NavigationSystemV1.K2_GetRandomLocationInNavigableRadius` (`self.K2_GetActorLocation`) 600.0 null null) null
        (:`then`
          (set `self.moving` true))
        (:`OnSuccess`
          (set `self.moving` true :!label _label))
        (:`OnFail`
          (goto _label))))))

(fn `UserConstructionScript`)